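; Procedural-generation chunk actor that builds an editable Paper2D tile map from its ChunkData at BeginPlay, laid flat at the chunk's position.
; CreateLayers adds one layer per mineral and biome enum value, mineral layers first, and maps each value to its layer index.
; Each data entry's flat index becomes X/Y, where AddTiles paints dirt or grass biome tiles and AddMinerals paints minerals, all using the iron ore tileset.
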(event EventBeginPlay
  (bind _sizeoftile (Variables|Default|GetSizeOfTile))
  (bind _chunkdata (Variables|Default|GetChunkData))
  (bind _chunkdata_2 (Variables|Default|GetChunkData))
  (Transformation|SetWorldTransform (Variables|Default|GetRenderComponent) (Math|Transform|MakeTransform (Math|Conversions|ToVector(Vector2D) (.position (Variables|Default|GetChunkData))) "0.000000,0.000000,-90.000000" "1.000000,1.000000,1.000000") false false)
  (Class|PaperTileMapComponent|CreateNewTileMap (Variables|Default|GetRenderComponent) (.sizex _chunkdata) (.sizey _chunkdata) (Math|Float|Truncate (.x _sizeoftile)) (Math|Float|Truncate (.y _sizeoftile)) 2.0 false)
  (Class|PaperTileMapComponent|MakeTileMapEditable (Variables|Default|GetRenderComponent))
  (bind (_newbiomelayer _newminerallayer) (CallFunction|CreateLayers))
  (Variables|Default|SetBiomeLayer _newbiomelayer)
  (Variables|Default|SetMineralLayer _newminerallayer)
  (Development|PrintString (Utilities|String|BuildString(Integer) "before loop, with length of: " "" (Utilities|Array|Length (.tiles _chunkdata_2))))
  (for (_array_element _array_index) (.tiles _chunkdata_2)
    (CallFunction|AddTiles (.tile _array_element) (Math|Integer|%(Integer) _array_index (.sizex _chunkdata_2)) (/ _array_index (.sizex _chunkdata_2)))
    (CallFunction|AddMinerals (.mineral _array_element) (Math|Integer|%(Integer) _array_index (.sizex _chunkdata_2)) (/ _array_index (.sizex _chunkdata_2))))
  (Development|PrintString (Utilities|String|BuildString(Integer) "" "success with data size y: " (.sizex _chunkdata_2))))

(fn ConstructionScript)

(fn CreateLayers
  ;[1 1 1] Mineral layer
  (bind _enumvalue (|ForEachE_Mineral)
    (:LoopBody
      (Utilities|Map|Add (LocalVariables|GetNewLocalMineralLayer) _enumvalue (LocalVariables|GetCount))
      (LocalVariables|SetCount (+ (LocalVariables|GetCount) 1))
      (Class|PaperTileMapComponent|AddNewLayer (Variables|Default|GetRenderComponent)))
    (:then
      ;[1 1 1] Biome layer
      (bind _enumvalue_2 (|ForEachE_Biome)
        (:LoopBody
          (Utilities|Map|Add (LocalVariables|GetNewLocalBiomeLayer) _enumvalue_2 (LocalVariables|GetCount))
          (LocalVariables|SetCount (+ (LocalVariables|GetCount) 1))
          (Class|PaperTileMapComponent|AddNewLayer (Variables|Default|GetRenderComponent)))
        (:then
          (return (LocalVariables|GetNewLocalBiomeLayer) (LocalVariables|GetNewLocalMineralLayer)))))))

(fn AddTiles
  (params (Tiles :type Map%20of%20E_Biome%20Enums%20to%20Integers :default "NewEnumerator0") (x :type Integer) (y :type Integer))
  (bind _keys (Utilities|Map|Keys Tiles))
  (for _array_element _keys
    (switch Utilities|FlowControl|Switch|SwitchonE_Biome _array_element
      (:NewEnumerator0
        (LocalVariables|SetUsedTileset "/Game/Graphics/Terrain/hr-dirt-1_TileSet.hr-dirt-1_TileSet"))
      (:NewEnumerator1
        (LocalVariables|SetUsedTileset "/Game/Graphics/Terrain/hr-grass-1_TileSet.hr-grass-1_TileSet")))
    (if (>= (.Value (Utilities|Map|Find (Variables|Default|GetBiomeLayer) _array_element)) 0)
      (Class|PaperTileMapComponent|SetTile (Variables|Default|GetRenderComponent) x y (.Value (Utilities|Map|Find (Variables|Default|GetBiomeLayer) _array_element)) (Class|TileMapBlueprintLibrary|MakeTile (.Value (Utilities|Map|Find Tiles _array_element)) (LocalVariables|GetUsedTileset)))))
  (return))

(fn AddMinerals
  (params (Tiles :type Map%20of%20E_Mineral%20Enums%20to%20Integers :default "NewEnumerator0") (x :type Integer) (y :type Integer))
  (bind _keys (Utilities|Map|Keys Tiles))
  (for _array_element _keys
    (switch Utilities|FlowControl|Switch|SwitchonE_Mineral _array_element
      (:NewEnumerator0
        (LocalVariables|SetUsedTileset "/Game/Graphics/Minerals/iron-ore_TileSet.iron-ore_TileSet")
        (if (>= (.Value (Utilities|Map|Find (Variables|Default|GetMineralLayer) _array_element)) 0)
          (Class|PaperTileMapComponent|SetTile (Variables|Default|GetRenderComponent) x y (.Value (Utilities|Map|Find (Variables|Default|GetMineralLayer) _array_element)) (Class|TileMapBlueprintLibrary|MakeTile (.Value (Utilities|Map|Find Tiles _array_element)) (LocalVariables|GetUsedTileset)))))))
  (return))