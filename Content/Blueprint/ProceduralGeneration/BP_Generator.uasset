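; BP_Generator procedurally builds a tile world of four chunks in a 2x2 layout meeting at the origin.
; The construction script creates a randomly seeded stream that drives all generation.
; GenerateChunk picks one random biome, fills tiles with random variants and rare minerals, and assigns an incrementing ID.
; DisplayChunk spawns each result as an attached BP_Chunk, with BeginPlay waiting a tick between chunks.
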(event EventBeginPlay
  (bind _newchunk (CallFunction|GenerateChunk))
  (CallFunction|DisplayChunk _newchunk)
  (Utilities|FlowControl|DelayUntilNextTick)
  (bind _newchunk_2 (CallFunction|GenerateChunk (* "(X=-1.000000,Y=0.000000)" (* (Math|Vector2D|MakeVector2D (Math|Conversions|ToFloat(Integer) (.SizeX (Utilities|Struct|BreakS_Chunk _newchunk))) (Math|Conversions|ToFloat(Integer) (.SizeY (Utilities|Struct|BreakS_Chunk _newchunk)))) "(X=32.000000,Y=32.000000)"))))
  (CallFunction|DisplayChunk _newchunk_2)
  (Utilities|FlowControl|DelayUntilNextTick)
  (bind _newchunk_3 (CallFunction|GenerateChunk (* "(X=0.000000,Y=-1.000000)" (* (Math|Vector2D|MakeVector2D (Math|Conversions|ToFloat(Integer) (.SizeX (Utilities|Struct|BreakS_Chunk _newchunk))) (Math|Conversions|ToFloat(Integer) (.SizeY (Utilities|Struct|BreakS_Chunk _newchunk)))) "(X=32.000000,Y=32.000000)"))))
  (CallFunction|DisplayChunk _newchunk_3)
  (Utilities|FlowControl|DelayUntilNextTick)
  (bind _newchunk_4 (CallFunction|GenerateChunk (* "(X=-1.000000,Y=-1.000000)" (* (Math|Vector2D|MakeVector2D (Math|Conversions|ToFloat(Integer) (.SizeX (Utilities|Struct|BreakS_Chunk _newchunk))) (Math|Conversions|ToFloat(Integer) (.SizeY (Utilities|Struct|BreakS_Chunk _newchunk)))) "(X=32.000000,Y=32.000000)"))))
  (CallFunction|DisplayChunk _newchunk_4))

(fn ConstructionScript
  (bind _output_get (Variables|Default|SetSeed (Math|Random|RandomInteger 10000000)))
  (Variables|Default|SetRandom (Math|Random|MakeRandomStream _output_get)))

(fn GenerateChunk
  (params (NewPosition :type Vector%202D%20Structure))
  (bind _chunk (LocalVariables|GetChunk))
  (bind _chunk_2 (LocalVariables|GetChunk))
  (LocalVariables|SetChunkBiome (Utilities|Enum|ByteToEnumE_Biome (Math|Conversions|ToByte(Integer) (Class|KismetMathLibrary|RandomIntegerfromStream (|GetNumEnumEntries) (Variables|Default|GetRandom)))))
  ;[1 1 1] Loop tile creation
  (for _index (range 0 (- (* (.sizex _chunk) (.sizey _chunk)) 1))
    (if (Class|KismetMathLibrary|RandomBoolwithWeightfromStream 0.01 (Variables|Default|GetRandom))
      (Utilities|Array|Add (.tiles _chunk_2) (Utilities|Struct|MakeS_Tile (Utilities|Map|MakeMap (LocalVariables|GetChunkBiome) (Math|Random|RandomIntegerinRangefromStream 320 575 (Variables|Default|GetRandom))) (Utilities|Map|MakeMap "NewEnumerator0" (Math|Random|RandomIntegerinRangefromStream 0 39 (Variables|Default|GetRandom)))))
      (else
        (Utilities|Array|Add (.tiles _chunk_2) (Utilities|Struct|MakeS_Tile (Utilities|Map|MakeMap (LocalVariables|GetChunkBiome) (Math|Random|RandomIntegerinRangefromStream 320 575 (Variables|Default|GetRandom))) "()")))))
  ;[1 1 1] Chunk ID
  (bind _output_get (Variables|Default|SetChunkIdIncrement (+ (Variables|Default|GetChunkIdIncrement) 1)))
  (return (Utilities|Struct|MakeS_Chunk _output_get NewPosition (.tiles (LocalVariables|GetChunk)) 128 128)))

(fn DisplayChunk
  (params (NewChunk :type S%20Chunk%20Structure))
  (bind _returnvalue (Game|SpawnActorfromClass "/Game/Blueprint/ProceduralGeneration/BP_Chunk.BP_Chunk_C" (Math|Transform|MakeTransform "0, 0, 0" "0, 0, 0" "1.000000,1.000000,1.000000") "AlwaysSpawn" 0 NewChunk 0))
  (Transformation|AttachActorToActor _returnvalue self "None" "KeepWorld" "KeepWorld" "KeepWorld" false))