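; BP_HR_AssemblingMachine2 is an assembling machine entity with a running state and an animated RenderComponent.
; StartRunning and StopRunning set the Running flag and play or stop the RenderComponent animation together.
; BeginPlay runs one timed cycle, starting the machine after a short delay and stopping it after another, with no production logic in this graph.
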(event Custom|StartRunning
  ;[1 1 1] Set running & Annimation
  (Variables|Default|SetRunning true)
  (Audio|Components|Audio|Play (Variables|Default|GetRenderComponent)))

(event Custom|StopRunning
  ;[1 1 1] Set running & Annimation
  (Variables|Default|SetRunning false)
  (Audio|Components|Audio|Stop (Variables|Default|GetRenderComponent)))

(event EventBeginPlay
  (Utilities|FlowControl|Delay 2.0)
  (CallFunction|StartRunning)
  (Utilities|FlowControl|Delay 2.0)
  (CallFunction|StopRunning))

(event Collision|EventActorBeginOverlap
  (params (OtherActor :type Actor%20Object%20Reference)))

(event EventTick
  (params (DeltaSeconds :type Float%20%28single-precision%29)))

(fn ConstructionScript)