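; Grid-sized in-world object actor whose footprint is defined as a number of cases (tiles).
; The construction script sizes the Tile box from half of SizeOfOneCase, as an integer vector, multiplied by SizeInCase in X and Y, keeping one case of height.
; It also resets the root's world rotation to zero, keeping X/Y location and scale while leaving Z at its default.
; The event graph holds no active logic.
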(event EventBeginPlay)

(event Collision|EventActorBeginOverlap
  (params (OtherActor :type Actor%20Object%20Reference)))

(event EventTick
  (params (DeltaSeconds :type Float%20%28single-precision%29)))

(fn ConstructionScript
  (bind _sizeofonecase (Variables|Default|GetSizeOfOneCase))
  (bind _defaultsceneroot (Variables|Default|GetDefaultSceneRoot))
  (bind _returnvalue (Transformation|GetWorldTransform _defaultsceneroot))
  (bind _returnvalue_2 (/ _sizeofonecase 2))
  ;[1 1 1] Set Size of tile
  (Components|Box|SetBoxExtent (Variables|Default|GetTile) (* (Utilities|Struct|MakeIntVector _returnvalue_2 _returnvalue_2 _returnvalue_2) (Math|Conversions|ToVector(Vector2D) (Variables|Default|GetSizeInCase) 1.0)) true)
  ;[1 1 1] Position rotation and default position
  (Transformation|SetWorldTransform _defaultsceneroot (Math|Transform|MakeTransform (Math|Vector|MakeVector (.x (.location _returnvalue)) (.y (.location _returnvalue)) 0.0) "0.000000,0.000000,0.000000" (.scale _returnvalue)) false true))